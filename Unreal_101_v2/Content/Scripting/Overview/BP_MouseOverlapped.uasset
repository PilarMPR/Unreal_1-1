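; BP_MouseOverlapped is an actor that shows its Name text component while the mouse cursor is over it and hides it when the cursor leaves.
; It caches the third-person character on BeginPlay.
; On hover, it sets the text's relative yaw once, intended to face the player, using a look-at from the text to the character's follow camera, both taken as relative locations.
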(event EventBeginPlay
  (bind _asbp_third_person_character (Utilities|Casting|CastToBP_ThirdPersonCharacter (Game|GetPlayerCharacter 0)))
  (Variables|Default|SetChar%20ref _asbp_third_person_character))

(event Collision|EventActorBeginOverlap
  (params (OtherActor :type Actor%20Object%20Reference)))

(event EventTick
  (params (DeltaSeconds :type Float%20%28single-precision%29)))

(event MouseInput|EventActorBeginCursorOver
  (bind _name (Variables|Default|GetName))
  ;[1 1 1] when cursor over actor, component text faces player
  ;;[1 1 1 1 14] in here we set the visibility depending on the cursor overlap
  (Rendering|SetVisibility (Variables|Default|GetName) true false)
  ;;[1 1 1] Set relative text rotation depending on player location so player always sees text
  (Transformation|SetRelativeRotation _name (Math|Rotator|MakeRotator 0.0 0.0 (.Yaw (Math|Rotator|BreakRotator (Math|Rotator|FindLookatRotation (Variables|/Script/Engine.SceneComponent|GetRelativeLocation _name) (Variables|/Script/Engine.SceneComponent|GetRelativeLocation (Variables|/Game/ThirdPerson/Blueprints/BP_ThirdPersonCharacter.BP_ThirdPersonCharacter_C|GetFollowCamera (Variables|Default|GetChar%20ref))))))) false false))

(event MouseInput|EventActorEndCursorOver
  ;[1 1 1] when cursor over actor, component text faces player
  ;;[1 1 1 1 14] in here we set the visibility depending on the cursor overlap
  (Rendering|SetVisibility (Variables|Default|GetName) false false))

(fn ConstructionScript)